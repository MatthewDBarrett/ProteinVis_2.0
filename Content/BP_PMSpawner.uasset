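; Spawner actor for a protein visualisation that loads two PDB multimers side by side at startup through BP_ProcessPDB, with fixed or random colours.
; It binds the Socket.IO "set-file" event to spawn further proteins by filename, hiding cylinder mesh actors after loading.
; Other message handlers, not bound here, spawn preset molecules or adjust MyMolecule's scale and rotation, filtered by station index except presets.
; Atom scale changes are deferred to Tick.
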(event `self.ReceiveBeginPlay`
  (`KismetSystemLibrary.Delay` 0.1)
  (`SocketIOClientComponent.BindEventToFunction` (`self.SocketIOClient`) "set-file" "SetFIle" null "/protein-vis" "USE_DEFAULT")
  (`self.GenerateFixedColours` (`self.useRandomColours`))
  (`|ExecutionSequence`
    (:`then_0`
      (bind _returnvalue (`|SpawnActorFromClass` "/Game/BP_ProcessPDB.BP_ProcessPDB_C" (`KismetMathLibrary.MakeTransform` (0.0 0.0 0.0)) "Undefined" "OverrideRootScale" null null))
      (`ProcessPDB.setFixedColours` _returnvalue (`self.FixedColours`))
      (`ProcessPDB.SetFolder` _returnvalue "Multimers")
      (`ProcessPDB.LoadPDBfromFile` _returnvalue (`self.FileName1`))
      (bind _returnvalue_2 (`ProcessPDB.GetMolecules` _returnvalue))
      (for _array_element _returnvalue_2
        (bind _asmy_molecule (cast `/Game/MyMolecule` _array_element))
        (`KismetArrayLibrary.Array_Add` (`self.Molecules`) _asmy_molecule)
        (bind _outactors (`GameplayStatics.GetAllActorsOfClass` "/Game/BP_CylinderISMA.BP_CylinderISMA_C"))
        (for _array_element_2 _outactors
          (`self.SetActorHiddenInGame` _array_element_2 true))))
    (:`then_1`
      (bind _returnvalue_3 (`|SpawnActorFromClass` "/Game/BP_ProcessPDB.BP_ProcessPDB_C" (`KismetMathLibrary.MakeTransform` (6000.0 0.0 0.0)) "Undefined" "OverrideRootScale" null null))
      (`ProcessPDB.setFixedColours` _returnvalue_3 (`self.FixedColours`))
      (`ProcessPDB.SetFolder` _returnvalue_3 "Multimers")
      (`ProcessPDB.LoadPDBfromFile` _returnvalue_3 (`self.FileName2`))
      (bind _returnvalue_4 (`ProcessPDB.GetMolecules` _returnvalue_3))
      (for _array_element_3 _returnvalue_4
        (bind _asmy_molecule_2 (cast `/Game/MyMolecule` _array_element_3))
        (`Molecule.SetPosition` _asmy_molecule_2 (6000.0 0.0 0.0))
        (`KismetArrayLibrary.Array_Add` (`self.Molecules`) _asmy_molecule_2)
        (bind _outactors_2 (`GameplayStatics.GetAllActorsOfClass` "/Game/BP_CylinderISMA.BP_CylinderISMA_C"))
        (for _array_element_4 _outactors_2
          (`self.SetActorHiddenInGame` _array_element_4 true))))))

(event `self.ReceiveTick`
  (params (DeltaSeconds :type "Float (single-precision)"))
  (if (`self.AtomSizeUpdated`)
    (`/Game/MyMolecule.UpdateAtomScale` (`self.MyMolecule`) (`self.UpdatedAtomScale`))
    (set `self.AtomSizeUpdated` false)))

(fn `ButtonPress`
  (params (Message :type "SIOJsonObject Object Reference"))
  (bind _returnvalue (`KismetMathLibrary.MakeTransform` (0.0 0.0 0.0)))
  (bind _returnvalue_2 (`KismetStringLibrary.Conv_DoubleToString` (`SIOJsonObject.GetNumberField` Message "value")))
  (`KismetSystemLibrary.PrintString` (`KismetStringLibrary.Concat_StrStr` "Pressed Button" _returnvalue_2))
  (switch `string` _returnvalue_2
    (:`1.0`
      (bind _returnvalue_3 (`|SpawnActorFromClass` "/Game/MyMolecule.MyMolecule_C" _returnvalue "Undefined" "OverrideRootScale" null null))
      (`Molecule.SetAtomSize` _returnvalue_3 0.7)
      (`Molecule.SetFileName` _returnvalue_3 "3nir"))
    (:`2.0`
      (bind _returnvalue_4 (`|SpawnActorFromClass` "/Game/MyMolecule.MyMolecule_C" _returnvalue "Undefined" "OverrideRootScale" null null))
      (`Molecule.SetAtomSize` _returnvalue_4 0.7)
      (`Molecule.SetFileName` _returnvalue_4 "6dvu"))))

(fn `GenerateFixedColours`
  (params (isRandom :type Boolean))
  (bind _fixedcolours (`self.FixedColours`))
  (if isRandom
    (for _ (range 21)
      (`KismetArrayLibrary.Array_Add` (`self.FixedColours`) (`KismetMathLibrary.MakeVector` (`KismetMathLibrary.RandomFloatInRange` 1.0 255.0) (`KismetMathLibrary.RandomFloatInRange` 1.0 255.0) (`KismetMathLibrary.RandomFloatInRange` 1.0 255.0))))
    (else
      (`KismetArrayLibrary.Array_Add` _fixedcolours (`KismetMathLibrary.MakeVector` 96.0 207.0 255.0))
      (`KismetArrayLibrary.Array_Add` _fixedcolours (`KismetMathLibrary.MakeVector` 105.0 71.0 255.0))
      (`KismetArrayLibrary.Array_Add` _fixedcolours (`KismetMathLibrary.MakeVector` 255.0 73.0 230.0)))))

(fn `SetFile`
  (params (Message :type Text))
  ;[0.4393 0.6714 1] Spawn Protein
  (`GameplayStatics.PlaySoundAtLocation` "/Game/Audio/computer_chirp.computer_chirp" (`self.K2_GetActorLocation`) (struct) 1.0 1.0 0.0 "/Game/Audio/Test_Attenuation.Test_Attenuation" null null)
  (bind _returnvalue (`|SpawnActorFromClass` "/Game/BP_ProcessPDB.BP_ProcessPDB_C" (`KismetMathLibrary.MakeTransform` (0.0 0.0 0.0)) "Undefined" "OverrideRootScale" null null))
  (`ProcessPDB.setFixedColours` _returnvalue (`self.FixedColours`))
  (`ProcessPDB.SetFolder` _returnvalue (`self.folderName`))
  (`ProcessPDB.LoadPDBfromFile` _returnvalue (`KismetTextLibrary.Conv_TextToString` Message))
  (bind _outactors (`GameplayStatics.GetAllActorsOfClass` "/Game/BP_CylinderISMA.BP_CylinderISMA_C"))
  (for _array_element _outactors
    (`self.SetActorHiddenInGame` _array_element true)))

(fn `SetFolderName`
  (params (FolderName :type String))
  (set `self.folderName` FolderName))

(fn `UpdateAtomScale`
  (params (Message :type "SIOJsonObject Object Reference"))
  (if (== (`self.BM_Index`) (`KismetStringLibrary.Conv_StringToInt` (`SIOJsonObject.GetStringField` Message "station")))
    (set `self.AtomSizeUpdated` true)
    (set `self.UpdatedAtomScale` (`SIOJsonObject.GetNumberField` Message "atomScale"))))

(fn `UpdateContRotation`
  (params (Message :type "SIOJsonObject Object Reference"))
  (if (== (`self.BM_Index`) (`KismetStringLibrary.Conv_StringToInt` (`SIOJsonObject.GetStringField` Message "station")))
    (`/Game/MyMolecule.UpdateProteinContRotation` (`self.MyMolecule`) (`SIOJsonObject.GetBoolField` Message "contRotation"))))

(fn `UpdateManualRotation`
  (params (Message :type "SIOJsonObject Object Reference"))
  (if (== (`self.BM_Index`) (`KismetStringLibrary.Conv_StringToInt` (`SIOJsonObject.GetStringField` Message "station")))
    (`/Game/MyMolecule.UpdateProteinRotation` (`self.MyMolecule`) (`SIOJLibrary.Conv_JsonValueToFloat` (`SIOJsonObject.GetField` Message "velX")) (`SIOJLibrary.Conv_JsonValueToFloat` (`SIOJsonObject.GetField` Message "velY")))))

(fn `UpdateProteinScale`
  (params (Message :type "SIOJsonObject Object Reference"))
  (if (== (`self.BM_Index`) (`KismetStringLibrary.Conv_StringToInt` (`SIOJsonObject.GetStringField` Message "station")))
    (`/Game/MyMolecule.UpdateScale` (`self.MyMolecule`) (`SIOJsonObject.GetNumberField` Message "proteinScale"))))

(fn `UserConstructionScript`)