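; BP_Protein loads PDB protein files through a spawned BP_ProcessPDB, passing it a generated random colour palette.
; It scales each molecule's atom and connection actors by the largest recorded protein size, then places them relative to the deprojected screen centre.
; CreateProtein lists molecules in UI_DesktopViewer with preset layouts for one to four entries.
; CreateProtein2 registers them with the alignment UI, offsetting each by the displayed count.
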(event `self.ReceiveBeginPlay`
  (`self.GenerateFixedColours` (`self.useRandomColours`))
  (`KismetSystemLibrary.Delay` 0.1)
  (bind _foundwidgets (`WidgetBlueprintLibrary.GetAllWidgetsOfClass` "/Game/Widgets/UI_DesktopViewer.UI_DesktopViewer_C"))
  (for _array_element _foundwidgets
    (set `self.UI_DesktopViewer` _array_element)
    (if (`self.ProgramStart`)
      (set `self.ProgramStart` false)
      (`KismetSystemLibrary.Delay` 0.1 :!label _label)
      (`self.ProcessProtein`))))

(event `WaitForProtein`
  (goto _label))

(event `WaitForProtein2`
  (`KismetSystemLibrary.Delay` 0.1)
  (`self.ProcessProtein2`))

(fn `AddToList`
  (bind _ui_desktopviewer (`self.UI_DesktopViewer`))
  (if (`KismetSystemLibrary.IsValid` _ui_desktopviewer)
    (for _array_element (`self.Molecules`)
      (bind _returnvalue (`Molecule.GetAtomsPointer` _array_element))
      (bind _asbp_instanced_static_mesh_actor (cast `/Game/BP_InstancedStaticMeshActor` _returnvalue))
      (`BlueprintMapLibrary.Map_Add` (`self.Atoms`) _array_element _asbp_instanced_static_mesh_actor)
      (bind _returnvalue_2 (`Molecule.GetConnectionsPointer` _array_element))
      (bind _asbp_cylinder_isma (cast `/Game/BP_CylinderISMA` _returnvalue_2))
      (`BlueprintMapLibrary.Map_Add` (`self.Connections`) _array_element _asbp_cylinder_isma))
    (`/Game/Widgets/UI_DesktopViewer.AddMoleculeToList` _ui_desktopviewer (`self.fileName`) (`self.Molecules`) (`self.Atoms`) (`self.Connections`))))

(fn `CreateProtein`
  (params (folderName :type String) (fileName :type String) (`UI Desktop` :type "/Game/Widgets/UI_DesktopViewer Object Reference"))
  (set `self.UI_DesktopViewer` `UI Desktop`)
  (`self.WaitForProtein`)
  (set `self.folderName` folderName)
  (set `self.fileName` fileName))

(fn `CreateProtein2`
  (params (folderName :type String) (fileName :type String) (`UI Desktop` :type "/Game/Widgets/UI_DesktopViewer Object Reference") (UI_MolAlignment :type "/Game/Widgets/Molecule_Alignment Object Reference"))
  (set `self.UI_DesktopViewer` `UI Desktop`)
  (set `self.moleculeAlignment` UI_MolAlignment)
  (`self.WaitForProtein2`)
  (set `self.folderName` folderName)
  (set `self.fileName` fileName))

(fn `GenerateFixedColours`
  (params (isRandom :type Boolean))
  (bind _fixedcolours (`self.FixedColours`))
  (if true
    (for _ (range 21)
      (`KismetArrayLibrary.Array_Add` (`self.FixedColours`) (`KismetMathLibrary.MakeVector` (`KismetMathLibrary.RandomFloatInRange` 1.0 255.0) (`KismetMathLibrary.RandomFloatInRange` 1.0 255.0) (`KismetMathLibrary.RandomFloatInRange` 1.0 255.0))))
    (else
      (`KismetArrayLibrary.Array_Add` _fixedcolours (`KismetMathLibrary.MakeVector` 96.0 207.0 255.0))
      (`KismetArrayLibrary.Array_Add` _fixedcolours (`KismetMathLibrary.MakeVector` 105.0 71.0 255.0))
      (`KismetArrayLibrary.Array_Add` _fixedcolours (`KismetMathLibrary.MakeVector` 255.0 73.0 230.0)))))

(fn `ProcessProtein`
  (bind _ui_desktopviewer (`self.UI_DesktopViewer`))
  (bind _returnvalue (`|SpawnActorFromClass` "/Game/BP_ProcessPDB.BP_ProcessPDB_C" (`KismetMathLibrary.MakeTransform` (0.0 0.0 0.0)) "Undefined" "OverrideRootScale" null null))
  (`ProcessPDB.setFixedColours` _returnvalue (`self.FixedColours`))
  (`ProcessPDB.SetFolder` _returnvalue (`self.folderName`))
  (`ProcessPDB.LoadPDBfromFile` _returnvalue (`self.fileName`))
  (bind _returnvalue_2 (`ProcessPDB.GetMolecules` _returnvalue))
  (`KismetArrayLibrary.Array_Clear` (`self.Molecules`))
  (for _array_element _returnvalue_2
    (bind _asmy_molecule (cast `/Game/MyMolecule` _array_element))
    (`KismetArrayLibrary.Array_Add` (`self.Molecules`) _asmy_molecule)
    (bind _returnvalue_3 (`Molecule.GetProteinSize` _asmy_molecule))
    (`KismetArrayLibrary.Array_Add` (`self.ProteinScales`) _returnvalue_3))
  (for _array_element_2 (`self.Molecules`)
    (`self.SetProteinScale` _array_element_2))
  (`self.AddToList`)
  (`self.SetPositionsOnSceen`)
  (if (`KismetSystemLibrary.IsValid` _ui_desktopviewer)
    (if (`Widget.IsVisible` _ui_desktopviewer)
      (`Widget.SetVisibility` (`/Game/Widgets/UI_DesktopViewer.CircularThrobber_219` _ui_desktopviewer) "Hidden"))))

(fn `ProcessProtein2`
  (bind _ui_desktopviewer (`self.UI_DesktopViewer`))
  (bind _molecules (`self.Molecules`))
  (bind _returnvalue (`|SpawnActorFromClass` "/Game/BP_ProcessPDB.BP_ProcessPDB_C" (`KismetMathLibrary.MakeTransform` (0.0 0.0 0.0)) "Undefined" "OverrideRootScale" null null))
  (`ProcessPDB.setFixedColours` _returnvalue (`self.FixedColours`))
  (`ProcessPDB.SetFolder` _returnvalue (`self.folderName`))
  (`ProcessPDB.LoadPDBfromFile` _returnvalue (`self.fileName`))
  (bind _returnvalue_2 (`ProcessPDB.GetMolecules` _returnvalue))
  (`KismetArrayLibrary.Array_Clear` (`self.Molecules`))
  (for _array_element _returnvalue_2
    (bind _asmy_molecule (cast `/Game/MyMolecule` _array_element))
    (`KismetArrayLibrary.Array_Add` (`self.Molecules`) _asmy_molecule)
    (bind _returnvalue_3 (`Molecule.GetProteinSize` _asmy_molecule))
    (`KismetArrayLibrary.Array_Add` (`self.ProteinScales`) _returnvalue_3))
  (for _array_element_2 _molecules
    (`self.SetProteinScale` _array_element_2))
  (bind _moleculeobject (`/Game/Widgets/Molecule_Alignment.addToDisplayedMolecules` (`self.moleculeAlignment`) _molecules (`self.fileName`)))
  (`self.SetPositions2` _moleculeobject)
  (if (`KismetSystemLibrary.IsValid` _ui_desktopviewer)
    (if (`Widget.IsVisible` _ui_desktopviewer)
      (`Widget.SetVisibility` (`/Game/Widgets/UI_DesktopViewer.CircularThrobber_219` _ui_desktopviewer) "Hidden"))))

(fn `SetPositions2`
  (params (moleculeObject :type "/Game/MoleculeObject Structure"))
  (`self.UpdatePosition` (`KismetMathLibrary.MakeVector` 500.0 (`KismetMathLibrary.Conv_IntToDouble` (+ (* (- (`KismetArrayLibrary.Array_Length` (`/Game/Widgets/Molecule_Alignment.displayedMolecules` (`self.moleculeAlignment`))) 1) 4000) 800)) -250.0) moleculeObject))

(fn `SetPositionsOnSceen`
  (bind _ui_desktopviewer (`self.UI_DesktopViewer`))
  (bind _moleculelist (`/Game/Widgets/UI_DesktopViewer.MoleculeList` _ui_desktopviewer))
  (if (`KismetSystemLibrary.IsValid` _ui_desktopviewer)
    (for (_array_element _array_index) (`ListView.GetListItems` _moleculelist)
      (bind _asudata (cast `/Game/UData` _array_element))
      (switch `int` (`ListView.GetNumItems` _moleculelist)
        (:`1`
          (switch `int` _array_index
            (:`0`
              (bind _data (`/Game/UData.Data` _asudata))
              (`self.UpdatePosition` (500.0 -1000.0 -250.0) _data))))
        (:`2`
          (switch `int` _array_index
            (:`0`
              (`self.UpdatePosition` (2500.0 -2000.0 -250.0) _data))
            (:`1`
              (`self.UpdatePosition` (-2500.0 -1000.0 -250.0) _data))))
        (:`3`
          (switch `int` _array_index
            (:`0`
              (`self.UpdatePosition` (2500.0 -4000.0 -2500.0) _data))
            (:`1`
              (`self.UpdatePosition` (-2500.0 -2000.0 -2500.0) _data))
            (:`2`
              (`self.UpdatePosition` (0.0 -3000.0 1500.0) _data))))
        (:`4`
          (switch `int` _array_index
            (:`0`
              (`self.UpdatePosition` (-3250.0 -4500.0 900.0) _data))
            (:`1`
              (`self.UpdatePosition` (3250.0 -6000.0 900.0) _data))
            (:`2`
              (`self.UpdatePosition` (-3250.0 -4500.0 -4800.0) _data))
            (:`3`
              (`self.UpdatePosition` (3250.0 -6000.0 -4800.0) _data))))))))

(fn `SetProteinScale`
  (params (`My Molecule` :type "/Game/MyMolecule Object Reference"))
  (bind _returnvalue (/ (`.MaxValue` (`KismetMathLibrary.MaxOfFloatArray` (`self.ProteinScales`))) 50.0))
  (bind _returnvalue_2 (`Molecule.GetAtomsPointer` `My Molecule`))
  (bind _returnvalue_3 (`Molecule.GetConnectionsPointer` `My Molecule`))
  (bind _rootcomponent (`Actor.RootComponent` _returnvalue_2))
  (`SceneComponent.SetWorldScale3D` _rootcomponent (/ (`SceneComponent.K2_GetComponentScale` _rootcomponent) _returnvalue))
  (bind _rootcomponent_2 (`Actor.RootComponent` _returnvalue_3))
  (`SceneComponent.SetWorldScale3D` _rootcomponent_2 (/ (`SceneComponent.K2_GetComponentScale` _rootcomponent_2) _returnvalue)))

(fn `UpdatePosition`
  (params (PositionAdjustment :type "Vector Structure") (Molecule :type "/Game/MoleculeObject Structure"))
  (bind _returnvalue (`GameplayStatics.GetPlayerController` 0))
  (bind (_sizex _sizey) (`PlayerController.GetViewportSize` _returnvalue))
  (bind (_worldlocation _worlddirection) (`PlayerController.DeprojectScreenPositionToWorld` _returnvalue (/ (`KismetMathLibrary.Conv_IntToDouble` _sizex) 2.0) (/ (`KismetMathLibrary.Conv_IntToDouble` _sizey) 2.0)))
  (for _array_element (`.Molecules_28_17B035D843845AFB21FCF693185486D4` (break `/Game/MoleculeObject` Molecule))
    (if (`KismetSystemLibrary.IsValid` _array_element)
      (`Molecule.SetPosition` _array_element (+ PositionAdjustment (+ _worldlocation (* _worlddirection 5000)))))))

(fn `UserConstructionScript`)